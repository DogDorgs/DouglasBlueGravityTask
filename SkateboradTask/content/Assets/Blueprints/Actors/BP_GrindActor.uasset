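; Spline grind rail that BP_SkaterCharacter players can ride to perform tricks.
; The construction script lays hidden spline meshes along the spline as overlap triggers, which start a server-called grind when the skater wants one.
; A timeline moves skater and grind audio along the spline from the nearest point, choosing direction by tangent-to-facing dot product.
; Releasing or finishing restores collision, launches the skater, clears the trick and re-arms after a delay.
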(event `self.ReceiveBeginPlay`
  ;[0.1227 0.5626 1] Assign an event for any instance to detect overlap
  (for _array_element (`self.SplineMeshes`)
    (add `PrimitiveComponent.OnComponentBeginOverlap` _array_element (`|CreateDelegate` :!event `Overlap`))))

(event `Overlap`
  (params (OverlappedComponent :type "PrimitiveComponent Object Reference") (OtherActor :type "Actor Object Reference") (OtherComp :type "PrimitiveComponent Object Reference") (OtherBodyIndex :type Integer) (bFromSweep :type Boolean) (SweepResult :type "HitResult Structure (by ref)"))
  ;[0.1227 0.5626 1] Assign an event for any instance to detect overlap
  (if (`self.Active`)
    (bind _asbp_skater_character (cast `/Game/Assets/Blueprints/Characters/BP_SkaterCharacter` OtherActor))
    (if (`/Game/Assets/Blueprints/Characters/BP_SkaterCharacter.bWantsToGrind` _asbp_skater_character)
      (`self.ServerStartGriding` _asbp_skater_character)
      (`/Engine/EditorBlueprintResources/StandardMacros.Can Execute Cosmetic Events`
        (:`True`
          (`/Game/Assets/Blueprints/Characters/BP_SkaterCharacter.TryToDoLocalTrick` _asbp_skater_character "NewEnumerator1" 1.0)
          (set `self.Active` false))))))

(event `ServerStartGriding`
  (params (Object :type "Object Object Reference"))
  ;[0 0.8439 1] Server event when player calls it
  (bind _asbp_skater_character (cast `/Game/Assets/Blueprints/Characters/BP_SkaterCharacter` Object))
  (if (and (not (`/Game/Assets/Blueprints/Characters/BP_SkaterCharacter.bIsGriding` _asbp_skater_character)) (`/Game/Assets/Blueprints/Characters/BP_SkaterCharacter.bWantsToGrind` _asbp_skater_character))
    (set `self.EntryVelocity` (`MovementComponent.Velocity` (`Character.CharacterMovement` _asbp_skater_character)))
    (bind _output_get (set `self.Character` _asbp_skater_character))
    (`self.StartGrinding` _output_get)
    (set `/Game/Assets/Blueprints/Characters/BP_SkaterCharacter.bIsGriding` true _asbp_skater_character)))

(event `StartGrinding`
  (params (Target :type "/Game/Assets/Blueprints/Characters/BP_SkaterCharacter Object Reference"))
  (bind _spline (`self.Spline`))
  (bind _spline_2 (`self.Spline`))
  (bind _grindtl (`self.GrindTL`))
  (bind _spline_3 (`self.Spline`))
  (bind _returnvalue (`SplineComponent.GetDistanceAlongSplineAtSplineInputKey` _spline_3 (`SplineComponent.FindInputKeyClosestToWorldLocation` _spline_3 (`self.K2_GetActorLocation` Target))))
  ;[0.1818 1 0] Actual Griding
  (`AudioComponent.SetVolumeMultiplier` (`self.Grind`) 1.0)
  (`TimelineComponent.SetPlayRate` _grindtl (/ 1.0 (/ (/ (`SplineComponent.GetSplineLength` _spline) (`SplineComponent.GetNumberOfSplinePoints` _spline)) 150.0)))
  (`TimelineComponent.SetPlaybackPosition` _grindtl (`KismetMathLibrary.MapRangeClamped` _returnvalue 0.0 (`SplineComponent.GetSplineLength` _spline_3) 0.0 1.0) false false)
  (if (> (`KismetMathLibrary.Dot_VectorVector` (`SplineComponent.GetTangentAtDistanceAlongSpline` _spline_3 _returnvalue "World") (`self.GetActorForwardVector` Target)) 0.0)
    (bind (_direction _alpha) (`Timeline|GrindTL` :!label _label)
      (:`Update`
        (if (`/Game/Assets/Blueprints/Characters/BP_SkaterCharacter.bWantsToGrind` Target)
          (`PrimitiveComponent.SetCollisionEnabled` (`Character.CapsuleComponent` Target) "QueryOnly")
          (`CharacterMovementComponent.SetMovementMode` (`Character.CharacterMovement` Target) "MOVE_None" 0)
          (bind (_returnvalue_x _returnvalue_y _returnvalue_z) (`KismetMathLibrary.BreakVector` (`SplineComponent.GetLocationAtTime` _spline_2 _alpha "World" true)))
          (bind _returnvalue_2 (`KismetMathLibrary.MakeVector` _returnvalue_x _returnvalue_y (+ _returnvalue_z 100.0)))
          (`SceneComponent.K2_SetWorldLocation` (`self.Grind`) _returnvalue_2 false true)
          (bind _returnvalue_3 (`KismetMathLibrary.ComposeRotators` (`SplineComponent.GetRotationAtTime` _spline_2 _alpha "World" true) (select `ETimelineDirection` _direction :`Backward` (struct :`Yaw` 180.0) :!type "Rotator Structure")))
          (`self.K2_SetActorLocationAndRotation` Target _returnvalue_2 _returnvalue_3 false true)
          (`Controller.SetControlRotation` (`Pawn.GetController` Target) _returnvalue_3)
          (else
            (`self.StopGriding`))))
      (:`Finished`
        (`self.EndGrind`)))
    (else
      (goto _label :!via `Reverse`))))

(event `StopGriding`
  ;[0.1818 1 0] Actual Griding
  (`self.EndGrind`)
  (goto _label :!via `Stop`))

(event `EndGrind`
  (bind _character (`self.Character`))
  (bind _playerstate (`Controller.PlayerState` (`Pawn.GetController` _character)))
  ;[1 0.1206 0] Ends griding and set the parameters back
  (`|ExecutionSequence`
    (:`then_0`
      (set `/Game/Assets/Blueprints/Characters/BP_SkaterCharacter.bIsGriding` false _character)
      (`PrimitiveComponent.SetCollisionEnabled` (`Character.CapsuleComponent` _character) "QueryAndPhysics")
      (`/Game/Assets/Blueprints/Characters/BP_SkaterCharacter.Ollie` _character true 0.0)
      (`CharacterMovementComponent.SetMovementMode` (`Character.CharacterMovement` _character) "MOVE_Falling" 0)
      (`/Game/Assets/Blueprints/Characters/BP_SkaterCharacter.ServerStopMontage` _character 0.5)
      (`Character.LaunchCharacter` _character (+ (* (`self.GetActorForwardVector` _character) 800.0) (0.0 0.0 900.0)) true true)
      (set `/Game/Assets/Blueprints/ActorComponents/AC_ScoreManager.CurrentTrick` "NewEnumerator0" (`self.GetComponentByClass` _playerstate "/Game/Assets/Blueprints/ActorComponents/AC_ScoreManager.AC_ScoreManager_C"))
      (message `/Game/Assets/Blueprints/GameMode/BPI_GameState.StopTrick` (`GameplayStatics.GetGameState`) _playerstate)
      (`AudioComponent.SetVolumeMultiplier` (`self.Grind`) 0.0))
    (:`then_1`
      (`KismetSystemLibrary.Delay` 0.4)
      (set `self.Active` true))))

(fn `Get Start and End Position And Tangent At Index`
  (params (Index :type Integer))
  (returns (StartPosition :type "Vector Structure") (StartTangent :type "Vector Structure") (EndPosition :type "Vector Structure") (EndTangent :type "Vector Structure"))
  (bind _spline (`self.Spline`))
  (bind _returnvalue (* (+ Index 1) (`self.SectionLenght`)))
  (bind _returnvalue_2 (* Index (`self.SectionLenght`)))
  (return (`SplineComponent.GetLocationAtDistanceAlongSpline` _spline _returnvalue_2 "Local") (`SplineComponent.GetTangentAtDistanceAlongSpline` _spline _returnvalue_2 "Local") (`SplineComponent.GetLocationAtDistanceAlongSpline` _spline _returnvalue "Local") (`SplineComponent.GetTangentAtDistanceAlongSpline` _spline _returnvalue "Local")))

(fn `UserConstructionScript`
  ;[1 1 1] Premade logic
  (bind _mesh (`self.Mesh`)
    (:`then`
      (bind (_returnvalue_min _returnvalue_max) (break `Box` (`StaticMesh.GetBoundingBox` _mesh)))
      (bind _returnvalue_x (`KismetMathLibrary.BreakVector` (- _returnvalue_max _returnvalue_min)))
      (set `self.SectionLenght` _returnvalue_x)
      (for _index (range (+ (`KismetMathLibrary.FFloor` (/ (`SplineComponent.GetSplineLength` (`self.Spline`)) _returnvalue_x)) 1))
        (bind _returnvalue (`AddComponent|NODE_AddSplineMeshComponent-0`))
        (`StaticMeshComponent.SetStaticMesh` _returnvalue (`self.Mesh`))
        (`SceneComponent.SetHiddenInGame` _returnvalue true true)
        (bind (_startposition _starttangent _endposition _endtangent) (`self.Get Start and End Position And Tangent At Index` _index))
        (`SplineMeshComponent.SetStartAndEnd` _returnvalue _startposition _starttangent _endposition _endtangent true)
        (`KismetArrayLibrary.Array_Add` (`self.SplineMeshes`) _returnvalue)))
    (:`else`)))