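; Game state for the skater game that routes trick scoring and combo events to each player's score manager.
; BeginPlay caches the row names of the DT_Tricks data table.
; AddScore turns the trick enum into a row name, fetches that row and passes it to the AC_ScoreManager component on the given PlayerState.
; StopTrick, CancelCombo and FinishCombo forward directly to the same component.
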(event `self.ReceiveBeginPlay`
  (bind _outrownames (`DataTableFunctionLibrary.GetDataTableRowNames` "/Game/Assets/DT/DT_Tricks.DT_Tricks"))
  (set `self.TricksNames` _outrownames))

(event `/Game/Assets/Blueprints/GameMode/BPI_GameState.AddScore`
  (params (Trick :type "/Game/Assets/DT/E_Tricks Enum" :default "NewEnumerator0") (PlayerState :type "PlayerState Object Reference"))
  (bind _tricksnames (`self.TricksNames`))
  (bind _returnvalue (`|GetDataTableRow` "/Game/Assets/DT/DT_Tricks.DT_Tricks" (`|GetArrayItem` _tricksnames (`KismetArrayLibrary.Array_Find` _tricksnames (`KismetStringLibrary.Conv_StringToName` (`|GetEnumeratorNameAsString` Trick)))))
    (:`then`
      (`/Game/Assets/Blueprints/ActorComponents/AC_ScoreManager.AddScoreToPlayer` (`self.GetComponentByClass` PlayerState "/Game/Assets/Blueprints/ActorComponents/AC_ScoreManager.AC_ScoreManager_C") _returnvalue))))

(event `/Game/Assets/Blueprints/GameMode/BPI_GameState.StopTrick`
  (params (PlayerState :type "PlayerState Object Reference"))
  (`/Game/Assets/Blueprints/ActorComponents/AC_ScoreManager.StopTrick` (`self.GetComponentByClass` PlayerState "/Game/Assets/Blueprints/ActorComponents/AC_ScoreManager.AC_ScoreManager_C")))

(event `/Game/Assets/Blueprints/GameMode/BPI_GameState.CancelCombo`
  (params (PlayerState :type "PlayerState Object Reference"))
  (`/Game/Assets/Blueprints/ActorComponents/AC_ScoreManager.CancelCombo` (`self.GetComponentByClass` PlayerState "/Game/Assets/Blueprints/ActorComponents/AC_ScoreManager.AC_ScoreManager_C")))

(event `/Game/Assets/Blueprints/GameMode/BPI_GameState.FinishCombo`
  (params (PlayerState :type "PlayerState Object Reference"))
  (`/Game/Assets/Blueprints/ActorComponents/AC_ScoreManager.FinishCombo` (`self.GetComponentByClass` PlayerState "/Game/Assets/Blueprints/ActorComponents/AC_ScoreManager.AC_ScoreManager_C")))

(fn `UserConstructionScript`)