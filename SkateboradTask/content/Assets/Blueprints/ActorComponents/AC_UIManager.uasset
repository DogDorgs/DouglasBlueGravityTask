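; Controller component that manages player UI, creating and removing the main HUD and adding a points widget.
; On BeginPlay it retries each tick until the PlayerState is valid, covering late availability on dedicated servers.
; Where cosmetic events can execute, it binds to the PlayerState's AC_ScoreManager and shows WBP_HUD.
; A score-added event creates WBP_Points for the owning player if none is valid.
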(event `self.ReceiveBeginPlay`
  (`self.CreateMainHUD`))

(event `CreateMainHUD`
  (bind _playerstate (`Controller.PlayerState` (cast `Controller` (`self.GetOwner`) :!pure true)))
  (`/Engine/EditorBlueprintResources/StandardMacros.IsValid` _playerstate :!label _label
    (:`Is Valid`
      (`/Engine/EditorBlueprintResources/StandardMacros.Can Execute Cosmetic Events`
        (:`True`
          (add `/Game/Assets/Blueprints/ActorComponents/AC_ScoreManager.ScoreAdded` (`Actor.GetComponentByClass` _playerstate "/Game/Assets/Blueprints/ActorComponents/AC_ScoreManager.AC_ScoreManager_C") (delegate `ScoreAdded_Event`))
          (bind _returnvalue (`|CreateWidget` "/Game/Assets/UI/Widgets/WBP_HUD.WBP_HUD_C"))
          (`UserWidget.AddToViewport` _returnvalue 0)
          (set `self.MainHUD` _returnvalue))))
    (:`Is Not Valid`
      (`KismetSystemLibrary.DelayUntilNextTick`) ; Wait for player state to be available on dedicated servers
      (goto _label))))

(event `ScoreAdded_Event`
  (params (ScoreAdded :type "Float (double-precision)"))
  (`self.PointsHUD`
    (:`then`)
    (:`else`
      (bind _returnvalue (`|CreateWidget` "/Game/Assets/UI/Widgets/WBP_Points.WBP_Points_C" (cast `PlayerController` (`self.GetOwner`) :!pure true)))
      (bind _output_get (set `self.PointsHUD` _returnvalue))
      (`UserWidget.AddToViewport` _output_get 0))))

(event `RemoveMainHUD`
  (bind _mainhud (`self.MainHUD`)
    (:`then`
      (`Widget.RemoveFromParent` _mainhud))
    (:`else`)))