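; Actor component that tracks a skater's trick score and combos, broadcasting changes through event dispatchers and OnRep functions.
; Tricks add to a pending score, either once or through a looping timer for held tricks, and append their names to the combo.
; A retriggerable delay, timed from BP_SkaterGameState, banks pending points multiplied by combo length.
; FinishCombo banks immediately, while CancelCombo discards pending points.
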(event `self.ReceiveBeginPlay`
  (bind _asbp_skater_game_state (cast `/Game/Assets/Blueprints/GameMode/BP_SkaterGameState` (`GameplayStatics.GetGameState`)))
  (set `self.MaxComboTimer` (`/Game/Assets/Blueprints/GameMode/BP_SkaterGameState.MaxComboTime` _asbp_skater_game_state)))

(event `FinishCombo`
  (bind _localcombocache (`self.LocalComboCache`))
  (`self.ComboFinished`)
  (set `self.PlayerScore` (+ (* (`self.ScoreToAdd`) (`KismetArrayLibrary.Array_Length` (`self.Combo`))) (`self.PlayerScore`)) :!label _label)
  (set `self.ScoreToAdd` 0.0)
  (`KismetArrayLibrary.Array_Clear` _localcombocache)
  (set `self.Combo` _localcombocache))

(event `AddScoreToPlayer`
  (params (`Trick ` :type "/Game/Assets/DT/S_Tricks Structure"))
  (bind ((`TrickName_2_50C4D6054C6A0CB48A8C0DA71E795073` _trickname) (`Loop_11_FC35D4FF4F33C4E517324EB3E01A86E8` _loop)) (break `/Game/Assets/DT/S_Tricks` `Trick `))
  (set `self.LastScore` (`self.PlayerScore`))
  (`KismetSystemLibrary.K2_ClearAndInvalidateTimerHandle` (`self.LoopHandle`))
  (if _loop
    (`self.SetTimerTrickPoints` `Trick `)
    (else
      (`self.UpdateScore` `Trick `)))
  (`KismetArrayLibrary.Array_Add` (`self.LocalComboCache`) _trickname)
  (set `self.Combo` (`self.LocalComboCache`))
  (`KismetSystemLibrary.RetriggerableDelay` (`self.MaxComboTimer`) :!label _label_2)
  (goto _label))

(event `ResetComboTimer`
  (goto _label_2))

(event `SetTimerTrickPoints`
  (params (Trick :type "/Game/Assets/DT/S_Tricks Structure"))
  (set `self.LoopTrick` Trick)
  (if (`KismetSystemLibrary.K2_TimerExistsHandle` (`self.LoopHandle`))
    (`KismetSystemLibrary.K2_ClearAndInvalidateTimerHandle` (`self.LoopHandle`)))
  (bind _returnvalue (`KismetSystemLibrary.K2_SetTimerDelegate` (delegate `Loop`) (`self.AddPointsRate`) true))
  (set `self.LoopHandle` _returnvalue))

(event `Loop`
  (`self.UpdateScore` (`self.LoopTrick`)))

(event `StopTrick`
  (`KismetSystemLibrary.K2_ClearAndInvalidateTimerHandle` (`self.LoopHandle`)))

(event `CancelCombo`
  (`self.ComboCanceled`)
  (set `self.ScoreToAdd` 0.0))

(fn `OnRep_Combo`
  (`self.ComboChanged` (`self.Combo`)))

(fn `OnRep_PlayerScore`
  (`self.ScoreChanged` (`self.PlayerScore`)))

(fn `UpdateScore`
  (params (Trick :type "/Game/Assets/DT/S_Tricks Structure"))
  (bind (_trickname _pointspersecond _mustbeonair _loop) (break `/Game/Assets/DT/S_Tricks` Trick))
  (bind _output_get (set `self.ScoreToAdd` (+ (select `bool` _loop :`false` _pointspersecond :`true` (* _pointspersecond (`self.AddPointsRate`))) (`self.ScoreToAdd`))))
  (set `self.CurrentTrick` _trickname)
  (`self.ScoreAdded` _output_get)
  (`self.ResetComboTimer`))